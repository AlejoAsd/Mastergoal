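; Player controller for Mastergoal that shows on-screen text messages to its player through a MensajeWidget.
; After login, the local controller creates the widget hidden and adds it to the viewport.
; ActualizarMensaje sets the widget text and makes it visible, then hides it after a short delay unless the message is flagged to stay forever.
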(event Custom|ClientPostLogin
  (CallFunction|SetupUI))

(event EventActualizarMensaje
  (params (Mensaje :type String) (Forever :type Boolean))
  ;[1 1 1] Mensaje
  (bind _asmensaje_widget (Utilities|Casting|CastToMensajeWidget (Variables|Default|GetWidgetMensaje)))
  (Rendering|Components|TextRender|SetText (Variables|/Game/Mastergoal/UI/HUD/MensajeWidget.MensajeWidget_C|GetMensaje _asmensaje_widget) (Utilities|Text|ToText(String) Mensaje))
  (bind _asmensaje_widget_2 (Utilities|Casting|CastToMensajeWidget (Variables|Default|GetWidgetMensaje)))
  (Widget|SetVisibility _asmensaje_widget_2 "Visible")
  (if (not Forever)
    (Utilities|FlowControl|Delay 4.0)
    (Widget|SetVisibility _asmensaje_widget_2 "Hidden")))

(event EventBeginPlay)

(event EventTick
  (params (DeltaSeconds :type Float%20%28single-precision%29)))

(fn ConstructionScript)

(fn SetupUI
  (if (Pawn|IsLocalPlayerController)
    (bind _returnvalue (UserInterface|CreateWidget "/Game/Mastergoal/UI/HUD/MensajeWidget.MensajeWidget_C" self))
    (Widget|SetVisibility _returnvalue "Hidden")
    (bind _output_get (Variables|Default|SetWidgetMensaje _returnvalue))
    (UserInterface|Viewport|AddtoViewport _output_get 0)))