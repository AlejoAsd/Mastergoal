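; Controller Blueprint that opens the in-game pause menu when P is pressed during the Game Screen state.
; It asks BP_MenuFlowGameInstance to switch to PauseScreen, toggling an IsGamePaused flag and input, with no engine pause call.
; Both toggle branches set PauseScreen.
; The CallResumeButton event re-enables input and clears the flag without changing the menu state.
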(event Custom|CallResumeButton
  ;[1 1 1] Pause Game/Access In-Game Menu
  (Input|EnableInput 0)
  (Variables|Default|SetIsGamePaused false))

(event Input|KeyboardEvents|P
  ;[1 1 1] Pause Game/Access In-Game Menu
  (:Pressed
    (bind _asbp_menu_flow_game_instance (Utilities|Casting|CastToBP_MenuFlowGameInstance (Game|GetGameInstance)))
    (switch Utilities|FlowControl|Switch|SwitchonEGameState (Variables|/Game/Blueprints/BP_MenuFlowGameInstance.BP_MenuFlowGameInstance_C|GetGameState _asbp_menu_flow_game_instance)
      (:NewEnumerator1
        (if (Variables|Default|GetIsGamePaused)
          (bind _asbp_menu_flow_game_instance_2 (Utilities|Casting|CastToBP_MenuFlowGameInstance (Game|GetGameInstance)))
          (Default|SetState _asbp_menu_flow_game_instance_2 "NewEnumerator6")
          (Input|EnableInput 0)
          (Variables|Default|SetIsGamePaused false)
          (else
            (Variables|Default|SetIsGamePaused true)
            (bind _asbp_menu_flow_game_instance_3 (Utilities|Casting|CastToBP_MenuFlowGameInstance (Game|GetGameInstance)))
            (Default|SetState _asbp_menu_flow_game_instance_3 "NewEnumerator6")
            (Input|DisableInput 0)))))))

(fn ConstructionScript)