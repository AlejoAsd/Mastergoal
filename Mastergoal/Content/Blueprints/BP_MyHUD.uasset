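; BP_MyHUD is a HUD Blueprint that relays video setting choices from option widgets to the video options menu screen.
; Separate events handle resolution, anti-aliasing, shadow, texture and effects quality.
; Each casts the stored screen widget to WidgetBP_VideoOptionScreen, writes the new value to its current-setting variable, then collapses its scroll box.
; The graph only updates menu state and layout; it applies no engine settings itself.
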(event Custom|SetNewResolution
  (params (NewRes :type Text))
  ;[1 1 1] Called from Screen Res Widget; Makes menu layout changes to Video options screen, when setting new resolution
  (bind _aswidget_bp_video_option_screen (Utilities|Casting|CastToWidgetBP_VideoOptionScreen (Variables|Default|GetVideoOptionsScreenWidget)))
  (Variables|/Game/UI/Widgets/WidgetBP_VideoOptionScreen.WidgetBP_VideoOptionScreen_C|SetCurrentScreenResolution _aswidget_bp_video_option_screen NewRes)
  (Default|CollapseScrollBox _aswidget_bp_video_option_screen))

(event Custom|SetNewTextureQuality
  (params (New%20Texture%20Quality :type Text))
  ;[1 1 1] Called from Textures Widget; Makes menu layout changes to Video options screen, when setting new texture quality
  (bind _aswidget_bp_video_option_screen (Utilities|Casting|CastToWidgetBP_VideoOptionScreen (Variables|Default|GetVideoOptionsScreenWidget)))
  (Variables|/Game/UI/Widgets/WidgetBP_VideoOptionScreen.WidgetBP_VideoOptionScreen_C|SetCurrentTextureQuality _aswidget_bp_video_option_screen New%20Texture%20Quality)
  (Default|CollapseScrollBox _aswidget_bp_video_option_screen))

(event Custom|SetNewEffectsQuality
  (params (New%20Effects%20Quality :type Text))
  ;[1 1 1] Called from Effects Widget; Makes menu layout changes to Video options screen, when setting new effects quality
  (bind _aswidget_bp_video_option_screen (Utilities|Casting|CastToWidgetBP_VideoOptionScreen (Variables|Default|GetVideoOptionsScreenWidget)))
  (Variables|/Game/UI/Widgets/WidgetBP_VideoOptionScreen.WidgetBP_VideoOptionScreen_C|SetCurrentEffectsQuality _aswidget_bp_video_option_screen New%20Effects%20Quality)
  (Default|CollapseScrollBox _aswidget_bp_video_option_screen))

(event Custom|SetNewShadowQuality
  (params (NewShadowQuality :type Text))
  ;[1 1 1] Called from Shadows Widget; Makes menu layout changes to Video options screen, when setting new shadow quality
  (bind _aswidget_bp_video_option_screen (Utilities|Casting|CastToWidgetBP_VideoOptionScreen (Variables|Default|GetVideoOptionsScreenWidget)))
  (Variables|/Game/UI/Widgets/WidgetBP_VideoOptionScreen.WidgetBP_VideoOptionScreen_C|SetCurrentShadowQuality _aswidget_bp_video_option_screen NewShadowQuality)
  (Default|CollapseScrollBox _aswidget_bp_video_option_screen))

(event Custom|SetNewAA
  (params (NewAA :type Text))
  ;[1 1 1] Called from AA Widget; Makes menu layout changes to Video options screen, when setting AA Level
  (bind _aswidget_bp_video_option_screen (Utilities|Casting|CastToWidgetBP_VideoOptionScreen (Variables|Default|GetVideoOptionsScreenWidget)))
  (Variables|/Game/UI/Widgets/WidgetBP_VideoOptionScreen.WidgetBP_VideoOptionScreen_C|SetCurrentAALevel _aswidget_bp_video_option_screen NewAA)
  (Default|CollapseScrollBox _aswidget_bp_video_option_screen))

(fn ConstructionScript)