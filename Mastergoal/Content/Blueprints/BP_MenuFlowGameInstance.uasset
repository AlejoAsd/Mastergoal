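; Game instance Blueprint that tracks a global game state and drives the flow between the main menu and the puzzle example level.
; It creates a loading screen widget on Init, and SetState broadcasts state changes, adding or removing that widget when the loading state is entered or left.
; LoadGameLevel and BackToMainMenu switch to the loading state, pause briefly, then open their map by name.
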(event Custom|LoadGameLevel
  (CallFunction|SetState "NewEnumerator3")
  (Utilities|FlowControl|Delay 0.2)
  (Game|OpenLevel(byName) "PuzzleExampleMap"))

(event Custom|BackToMainMenu
  (CallFunction|SetState "NewEnumerator3")
  (Utilities|FlowControl|Delay 2.0)
  (Game|OpenLevel(byName) "/Game/Maps/MainMenu_Map"))

(event Custom|SetState
  (params (NewState :type EGameState%20Enum :default "NewEnumerator0"))
  ;[1 1 1] Handle Game State change and Dispatch State change event
  (if (not (== (Variables|Default|GetGameState) NewState))
    (Variables|Default|SetOldState (Variables|Default|GetGameState))
    (Variables|Default|SetGameState NewState)
    (Default|CallStateChanged (Variables|Default|GetOldState) (Variables|Default|GetGameState))
    (Utilities|FlowControl|Sequence
      (:then_0
        (switch Utilities|FlowControl|Switch|SwitchonEGameState (Variables|Default|GetOldState)
          (:NewEnumerator3
            (Widget|RemovefromParent (Variables|Default|GetLoadingUI)))))
      (:then_1
        (switch Utilities|FlowControl|Switch|SwitchonEGameState (Variables|Default|GetGameState)
          (:NewEnumerator3
            (UserInterface|Viewport|AddtoViewport (Variables|Default|GetLoadingUI) 0)))))))

(event EventInit
  (bind _returnvalue (UserInterface|CreateWidget "/Game/UI/Widgets/loadingScreen.loadingScreen_C"))
  (Variables|Default|SetLoadingUI _returnvalue))